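; BP_Lighthouse is an actor that tracks a TotalSolas pool, which drops when the lighthouse takes damage and rises through GainSolas.
; Both paths look up BP_RoundManager for active round modifiers.
; AttackIncreaseActive adds one to incoming damage, while HalfSolasActive halves gains after adding one.
; Damage clamps the pool at zero, and every change prints the new total.
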(event `Damage Lighthouse`
  (params (`Damage Dealt` :type Integer))
  (bind _returnvalue (`GameplayStatics.GetActorOfClass` "/Game/Blueprints/BP_RoundManager.BP_RoundManager_C"))
  (if (`/Game/Blueprints/BP_RoundManager.AttackIncrease_Active` _returnvalue)
    (bind _output_get (set `self.totalSolas` (- (`self.totalSolas`) (+ `Damage Dealt` 1))))
    (if (< _output_get 0)
      (set `self.totalSolas` 0))
    (`KismetSystemLibrary.PrintString` (`KismetStringLibrary.Conv_IntToString` (`self.totalSolas`)))
    (else
      (bind _output_get_2 (set `self.totalSolas` (- (`self.totalSolas`) `Damage Dealt`)))
      (if (< _output_get_2 0)
        (set `self.totalSolas` 0))
      (`KismetSystemLibrary.PrintString` (`KismetStringLibrary.Conv_IntToString` (`self.totalSolas`))))))

(fn `gainSolas`
  (params (solasGained :type Integer))
  (bind _returnvalue (`GameplayStatics.GetActorOfClass` "/Game/Blueprints/BP_RoundManager.BP_RoundManager_C"))
  (if (`/Game/Blueprints/BP_RoundManager.HalfSolas_Active` _returnvalue)
    (bind _output_get (set `self.totalSolas` (+ (/ (+ solasGained 1) 2) (`self.totalSolas`))))
    (`KismetSystemLibrary.PrintString` (`KismetStringLibrary.Conv_IntToString` _output_get))
    (else
      (bind _output_get_2 (set `self.totalSolas` (+ solasGained (`self.totalSolas`))))
      (`KismetSystemLibrary.PrintString` (`KismetStringLibrary.Conv_IntToString` _output_get_2)))))

(fn `UserConstructionScript`)