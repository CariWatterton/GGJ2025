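; Round manager that drives the monster's turns in a three-lane wave game and shows an end screen once its actions and the lanes are exhausted.
; TriggerRound plays PlayArea wave animations, while Roundlogic fires the Keeper's Kelpie ability, advances waves and updates the round tracker.
; Monster actions draw randomly without repeats: basic ones spawn waves, periodic skull ones enable lasting passives like double movement or stronger attacks.
; Nessie's passive lowers wave power.
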(event `self.ReceiveBeginPlay`
  (bind _playarea (`self.playArea`))
  (`self.Start Game`)
  (set `/Game/UI/HUD/PlayArea.RoundManager` self _playarea)
  (`/Game/UI/HUD/PlayArea.BindEvent` _playarea)
  (add `/Game/UI/Pieces/BP_Keeper.NessieAbility` (`self.keeper`) (`|CreateDelegate` :!event `NessiePassive`)))

(event `Trigger Round`
  (bind _playarea (`self.playArea`))
  (if (`self.IsFirstRound`)
    (set `self.IsFirstRound` false)
    (`self.Roundlogic`)
    (elif (`self.DoubleProjectileSpeed_Active`)
      (`UserWidget.PlayAnimationForward` _playarea (`/Game/UI/HUD/PlayArea.MoveWaves_TwiceHalf` _playarea) 1.0 true)
      (else
        (`UserWidget.PlayAnimationForward` _playarea (`/Game/UI/HUD/PlayArea.MoveWaves` _playarea) 1.0 true :!label _label)))))

(event `Start Game`
  (`self.Trigger Round`))

(event `SecondWave`
  (goto _label))

(event `ResolveFirstHalfOfDoubleWave`
  (`/Game/UI/HUD/PlayArea.ProgressWaves` (`self.playArea`)))

(event `Roundlogic`
  (bind _playarea (`self.playArea`))
  (bind _keeper (`self.keeper`))
  (`/Engine/EditorBlueprintResources/StandardMacros.IsValid` _keeper
    (:`Is Valid`
      (`/Game/UI/Pieces/BP_Keeper.KelpieAbility` _keeper))
    (:`Is Not Valid`
      _))
  (if (`self.DoubleProjectileSpeed_Active`)
    _
    (else
      _))
  (`/Game/UI/HUD/PlayArea.ProgressWaves` _playarea)
  (`/Game/UI/HUD/PlayArea.CheckLanes` _playarea)
  (if (and (`self.outOfSkullActions`) (`self.outOfBasicActions`))
    (if (`/Game/UI/HUD/PlayArea.lanesAreEmpty` (`self.playArea`))
      (`self.End of Game`))
    (else
      (bind _result (`/Engine/EditorBlueprintResources/StandardMacros.IncrementInt` (`self.roundCounter`))
        (:`  `
          (if (> (mod (/ _result (`self.skullRounds`)) 1.0) 0.0)
            (`self.basic_MonsterAction`)
            (else
              (`self.skull_MonsterAction`)))
          (`/Game/UI/Pieces/MonsterTurnTracker.UpdateNextAction` (`self.RoundTrackerUI`) (`self.roundCounter`)))))))

(event `End of Game`
  (set `self.endGame` true)
  (bind _returnvalue (`|CreateWidget` "/Game/UI/Menus/EndGameScreen.EndGameScreen_C"))
  (`UserWidget.AddToViewport` _returnvalue 0))

(fn `basic_MonsterAction`
  (bind _playarea (`self.playArea`))
  (bind _basewavepower (`self.BaseWavePower`))
  (bind _basewavepoweralllanes (`self.BaseWavePowerAllLanes`))
  (bind _basicmonsteractions (`self.basicMonsterActions`))
  (bind _output_get (set `self.basicActionInt` (`KismetArrayLibrary.Array_Random` (`self.basicMonsterActions`))))
  (switch `int` _output_get
    (:`0`
      (`/Game/UI/HUD/PlayArea.Add To Lane` _playarea 0 _basewavepower))
    (:`1`
      (`/Game/UI/HUD/PlayArea.Add To Lane` _playarea 0 _basewavepower))
    (:`2`
      (`/Game/UI/HUD/PlayArea.Add To Lane` _playarea 1 _basewavepower))
    (:`3`
      (`/Game/UI/HUD/PlayArea.Add To Lane` _playarea 1 _basewavepower))
    (:`4`
      (`/Game/UI/HUD/PlayArea.Add To Lane` _playarea 2 _basewavepower))
    (:`5`
      (`/Game/UI/HUD/PlayArea.Add To Lane` _playarea 2 _basewavepower))
    (:`6`
      (`/Game/UI/HUD/PlayArea.Add To Lane` _playarea 0 _basewavepoweralllanes)
      (`/Game/UI/HUD/PlayArea.Add To Lane` _playarea 1 _basewavepoweralllanes)
      (`/Game/UI/HUD/PlayArea.Add To Lane` _playarea 2 _basewavepoweralllanes))
    (:`7`
      (`/Game/UI/HUD/PlayArea.Add To Lane` _playarea 0 _basewavepoweralllanes)
      (`/Game/UI/HUD/PlayArea.Add To Lane` _playarea 1 _basewavepoweralllanes)
      (`/Game/UI/HUD/PlayArea.Add To Lane` _playarea 2 _basewavepoweralllanes)))
  (`KismetArrayLibrary.Array_RemoveItem` _basicmonsteractions (`self.basicActionInt`))
  (if (`KismetArrayLibrary.Array_IsEmpty` _basicmonsteractions)
    (set `self.outOfBasicActions` true)))

(fn `BindEvents`
  (bind _playarea (`self.playArea`))
  (bind _movewaves_twicehalf (`/Game/UI/HUD/PlayArea.MoveWaves_TwiceHalf` _playarea))
  (`UserWidget.BindToAnimationFinished` _playarea (`/Game/UI/HUD/PlayArea.MoveWaves` _playarea) (`|CreateDelegate` :!event `Roundlogic`))
  (`UserWidget.BindToAnimationFinished` _playarea _movewaves_twicehalf (`|CreateDelegate` :!event `ResolveFirstHalfOfDoubleWave`))
  (`UserWidget.BindToAnimationFinished` _playarea _movewaves_twicehalf (`|CreateDelegate` :!event `SecondWave`)))

(fn `NessiePassive`
  (`/Engine/EditorBlueprintResources/StandardMacros.DecrementInt` (`self.BaseWavePower`)
    (:`  `
      (`/Engine/EditorBlueprintResources/StandardMacros.DecrementInt` (`self.BaseWavePowerAllLanes`)
        (:`  `
          (`self.RebuildWaveVisuals` -1))))))

(fn `skull_AttackIncrease`
  (params (RandomAction :type Integer))
  (bind _skullmonsteraction (`self.skullMonsterAction`))
  (set `self.AttackIncrease_Active` true)
  (`KismetArrayLibrary.Array_RemoveItem` _skullmonsteraction RandomAction)
  (if (`KismetArrayLibrary.Array_IsEmpty` _skullmonsteraction)
    (set `self.outOfSkullActions` true))
  (`/Engine/EditorBlueprintResources/StandardMacros.IncrementInt` (`self.BaseWavePower`)
    (:`  `
      (`/Engine/EditorBlueprintResources/StandardMacros.IncrementInt` (`self.BaseWavePowerAllLanes`)
        (:`  `
          (`self.RebuildWaveVisuals` 1))))))

(fn `skull_DoubleProjectile`
  (params (RandomAction :type Integer))
  (bind _skullmonsteraction (`self.skullMonsterAction`))
  (set `self.DoubleProjectileSpeed_Active` true)
  (`KismetArrayLibrary.Array_RemoveItem` _skullmonsteraction RandomAction)
  (if (`KismetArrayLibrary.Array_IsEmpty` _skullmonsteraction)
    (set `self.outOfSkullActions` true)))

(fn `skull_ExtinguishGatherers`
  (params (RandomAction :type Integer))
  (bind _skullmonsteraction (`self.skullMonsterAction`))
  (set `self.ExtinguishGathers_Active` true)
  (`KismetArrayLibrary.Array_RemoveItem` _skullmonsteraction RandomAction)
  (if (`KismetArrayLibrary.Array_IsEmpty` _skullmonsteraction)
    (set `self.outOfSkullActions` true)))

(fn `skull_HalfSolas`
  (params (RandomAction :type Integer))
  (bind _skullmonsteraction (`self.skullMonsterAction`))
  (set `self.HalfSolas_Active` true)
  (`KismetArrayLibrary.Array_RemoveItem` _skullmonsteraction RandomAction)
  (if (`KismetArrayLibrary.Array_IsEmpty` _skullmonsteraction)
    (set `self.outOfSkullActions` true)))

(fn `skull_MonsterAction`
  (locals (currentSkullAction :type Integer :default 0))
  (bind _output_get (set `self.skullActionInt` (`KismetArrayLibrary.Array_Random` (`self.skullMonsterAction`))))
  (`/Game/UI/Pieces/BP_MonsterPassiveUI.AddPassive` (`self.MonsterPassivesUI`) _output_get)
  (switch `int` _output_get
    (:`0`
      (`self.skull_HalfSolas` _output_get))
    (:`1`
      (`self.skull_DoubleProjectile` _output_get))
    (:`2`
      (`self.skull_ExtinguishGatherers` _output_get))
    (:`3`
      (`self.skull_AttackIncrease` _output_get))))

(fn `UserConstructionScript`)